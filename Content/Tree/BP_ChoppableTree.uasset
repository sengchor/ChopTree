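; BP_ChoppableTree is a tree actor that weakens with each Chop call and then gets cut in two.
; The construction script copies its static mesh into a procedural mesh, and early chops raise a Hardness scalar on a dynamic material.
; Once the chop value reaches the threshold, it swaps to the procedural mesh, slices it along a tilted plane with capped halves and enables physics on the mesh.
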(event EventBeginPlay
  (bind _returnvalue (Rendering|Material|CreateDynamicMaterialInstance "/Game/Tree/M_Tree_Inst.M_Tree_Inst" "None" "None" :!class /Script/Engine.KismetMaterialLibrary))
  (bind _output_get (Variables|Default|SetMaterial _returnvalue))
  (Rendering|Material|SetMaterial (Variables|Default|GetStaticMesh) 0 _output_get)
  (Collision|SetCollisionEnabled (Variables|Default|GetProceduralMesh) "QueryAndPhysics"))

(event Collision|EventActorBeginOverlap
  (params (OtherActor :type Actor%20Object%20Reference)))

(event EventTick
  (params (DeltaSeconds :type Float%20%28single-precision%29)))

(event EventChop
  (bind _staticmesh (Variables|Default|GetStaticMesh))
  (bind _proceduralmesh (Variables|Default|GetProceduralMesh))
  (bind _returnvalue (Transformation|GetWorldLocation _staticmesh))
  (if (>= (Variables|Default|Getchopvalue) 0.4)
    (Development|PrintString "Slice" true true "(R=1.000000,G=0.000000,B=0.000000,A=1.000000)")
    (Rendering|SetVisibility (Variables|Default|GetStaticMesh) false false)
    (Rendering|SetVisibility (Variables|Default|GetProceduralMesh) true false)
    (Class|KismetProceduralMeshLibrary|SliceProceduralMesh _proceduralmesh (Math|Vector|MakeVector (.x _returnvalue) (.y _returnvalue) (+ (.z _returnvalue) 1.1e+02)) (Math|Vector|MakeVector 0.2 0.2 1.0) true "UseLastSectionForCap" "/Game/Megascans/Surfaces/Wood_qklp2op0/MI_Wood_qklp2op0_2K.MI_Wood_qklp2op0_2K")
    (Physics|SetSimulatePhysics _proceduralmesh true)
    (Physics|SetEnableGravity _proceduralmesh true)
    (Rendering|Material|SetMaterial (Variables|Default|GetProceduralMesh) 0 "/Game/Megascans/3D_Assets/Blackened_Tree_Trunk_vclpbigga/MI_Blackened_Tree_Trunk_vclpbigga_2K.MI_Blackened_Tree_Trunk_vclpbigga_2K")
    (else
      (Development|PrintString "Chop")
      (bind _output_get (Variables|Default|Setchopvalue (+ (Variables|Default|Getchopvalue) 0.2)))
      (Rendering|Material|SetScalarParameterValue (Variables|Default|GetMaterial) "Hardness" _output_get :!class /Script/Engine.MaterialInstanceDynamic))))

(fn ConstructionScript
  (Class|KismetProceduralMeshLibrary|CopyProceduralMeshfromStaticMeshComponent (Variables|Default|GetStaticMesh) 0 (Variables|Default|GetProceduralMesh) false))

(fn IsChoppable?
  (return true))